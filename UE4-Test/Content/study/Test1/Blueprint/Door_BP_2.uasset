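; A double door Blueprint whose two leaves swing open and closed when clicked or when the 2 key is pressed.
; A Box overlap opens a Gate and enables input, and leaving it closes both; either overlap event shows the mouse cursor, which is never hidden again.
; Input through the Gate drives a FlipFlop that plays or reverses one Timeline, lerping both leaves' yaw in opposite directions.
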(event OnComponentBeginOverlap(Box)
  (params (OverlappedComponent :type Primitive%20Component%20Object%20Reference) (OtherActor :type Actor%20Object%20Reference) (OtherComp :type Primitive%20Component%20Object%20Reference) (OtherBodyIndex :type Integer) (bFromSweep :type Boolean) (SweepResult :type Hit%20Result%20Structure%20%28by%20ref%29))
  (bind _returnvalue (Game|GetPlayerController 0))
  (Variables|/Script/Engine.PlayerController|SetbShowMouseCursor _returnvalue true)
  (Input|EnableInput _returnvalue)
  (Utilities|FlowControl|Gate true) ; enters at Open
)

(event OnComponentEndOverlap(Box)
  (params (OverlappedComponent :type Primitive%20Component%20Object%20Reference) (OtherActor :type Actor%20Object%20Reference) (OtherComp :type Primitive%20Component%20Object%20Reference) (OtherBodyIndex :type Integer))
  (bind _returnvalue (Game|GetPlayerController 0))
  (Variables|/Script/Engine.PlayerController|SetbShowMouseCursor _returnvalue true)
  (Input|DisableInput _returnvalue)
  (Utilities|FlowControl|Gate true) ; enters at Close
)

(event OnClicked(Door)
  (params (TouchedComponent :type Primitive%20Component%20Object%20Reference) (ButtonPressed :type Key%20Structure))
  (Utilities|FlowControl|Gate true
    (:Exit
      (Utilities|FlowControl|FlipFlop
        (:A
          (bind _新建轨道_0 (Timeline|时间轴_0 Play)
            (:Update
              (Transformation|SetRelativeRotation (Variables|Default|GetDoor) (Math|Rotator|MakeRotator 0.0 0.0 (Math|Float|Lerp -1.8e+02 -105.0 _新建轨道_0)) false false)
              (Transformation|SetRelativeRotation (Variables|Default|GetDoor1) (Math|Rotator|MakeRotator 0.0 0.0 (Math|Float|Lerp 0.0 -75.0 _新建轨道_0)) false false))))
        (:B
          (Timeline|时间轴_0 Reverse))))))

(event OnClicked(Door1)
  (params (TouchedComponent :type Primitive%20Component%20Object%20Reference) (ButtonPressed :type Key%20Structure))
  (Utilities|FlowControl|Gate true
    (:Exit
      (Utilities|FlowControl|FlipFlop
        (:A
          (bind _新建轨道_0 (Timeline|时间轴_0 Play)
            (:Update
              (Transformation|SetRelativeRotation (Variables|Default|GetDoor) (Math|Rotator|MakeRotator 0.0 0.0 (Math|Float|Lerp -1.8e+02 -105.0 _新建轨道_0)) false false)
              (Transformation|SetRelativeRotation (Variables|Default|GetDoor1) (Math|Rotator|MakeRotator 0.0 0.0 (Math|Float|Lerp 0.0 -75.0 _新建轨道_0)) false false))))
        (:B
          (Timeline|时间轴_0 Reverse))))))

(event EventBeginPlay)

(event Collision|EventActorBeginOverlap
  (params (OtherActor :type Actor%20Object%20Reference)))

(event EventTick
  (params (DeltaSeconds :type Float%20%28single-precision%29)))

(event Input|KeyboardEvents|2
  (params (Key :type Key%20Structure))
  (:Pressed
    (Utilities|FlowControl|Gate true
      (:Exit
        (Utilities|FlowControl|FlipFlop
          (:A
            (bind _新建轨道_0 (Timeline|时间轴_0 Play)
              (:Update
                (Transformation|SetRelativeRotation (Variables|Default|GetDoor) (Math|Rotator|MakeRotator 0.0 0.0 (Math|Float|Lerp -1.8e+02 -105.0 _新建轨道_0)) false false)
                (Transformation|SetRelativeRotation (Variables|Default|GetDoor1) (Math|Rotator|MakeRotator 0.0 0.0 (Math|Float|Lerp 0.0 -75.0 _新建轨道_0)) false false))))
          (:B
            (Timeline|时间轴_0 Reverse)))))))

(fn ConstructionScript)