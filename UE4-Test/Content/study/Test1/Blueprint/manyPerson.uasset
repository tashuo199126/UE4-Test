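; Blueprint that switches player control among five targets, apparently characters or pawns, each time the 1 key is pressed.
; A looping, non-random MultiGate picks the next target, blends the player controller's view to it with a cubic ease, then possesses it once the blend delay ends.
; The 判断镜头 flag blocks further presses until that transition completes.
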(event EventBeginPlay)

(event Collision|EventActorBeginOverlap
  (params (OtherActor :type Actor%20Object%20Reference)))

(event EventTick
  (params (DeltaSeconds :type Float%20%28single-precision%29)))

(event Input|KeyboardEvents|1
  (params (Key :type Key%20Structure :default "None"))
  (bind _returnvalue (Game|GetPlayerController 0))
  (bind _returnvalue_2 (Game|GetPlayerController 0))
  (:Pressed
    (if (not (Variables|Default|Get判断镜头))
      (Variables|Default|Set判断镜头 true)
      (Utilities|FlowControl|MultiGate false true -1
        (:Out%200
          (Game|Player|SetViewTargetwithBlend _returnvalue "Literal" 2.0 "VTBlend_Cubic" 0.0 false)
          (Utilities|FlowControl|Delay 2.0)
          (Pawn|Possess _returnvalue_2 "Literal")
          (Variables|Default|Set判断镜头 false))
        (:Out%201
          (Game|Player|SetViewTargetwithBlend _returnvalue "Literal" 2.0 "VTBlend_Cubic" 0.0 false)
          (Utilities|FlowControl|Delay 2.0)
          (Pawn|Possess _returnvalue_2 "Literal")
          (Variables|Default|Set判断镜头 false))
        (:Out%202
          (Game|Player|SetViewTargetwithBlend _returnvalue_2 "Literal" 2.0 "VTBlend_Cubic" 0.0 false)
          (Utilities|FlowControl|Delay 2.0)
          (Pawn|Possess _returnvalue_2 "Literal")
          (Variables|Default|Set判断镜头 false))
        (:Out%203
          (Game|Player|SetViewTargetwithBlend _returnvalue_2 "Literal" 2.0 "VTBlend_Cubic" 0.0 false)
          (Utilities|FlowControl|Delay 2.0)
          (Pawn|Possess _returnvalue_2 "Literal")
          (Variables|Default|Set判断镜头 false))
        (:Out%204
          (Game|Player|SetViewTargetwithBlend _returnvalue_2 "Literal" 2.0 "VTBlend_Cubic" 0.0 false)
          (Utilities|FlowControl|Delay 2.0)
          (Pawn|Possess _returnvalue_2 "Literal")
          (Variables|Default|Set判断镜头 false))))))

(fn ConstructionScript)