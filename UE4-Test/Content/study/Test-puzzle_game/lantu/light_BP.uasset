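; Light_BP is a puzzle light actor that the player switches on with F while inside its trigger box.
; Box overlap by the ThirdPersonCharacter toggles input and a Gate, showing a text prompt if the light is unlit.
; Lighting reveals the SpotLight, then checks every Light_BP instance's lit flag.
; When all are lit, a "ce" console command fires the 打开关卡机关 (open level mechanism) event in the Level Blueprint.
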(event OnComponentBeginOverlap(Box)
  (params (OverlappedComponent :type Primitive%20Component%20Object%20Reference) (OtherActor :type Actor%20Object%20Reference) (OtherComp :type Primitive%20Component%20Object%20Reference) (OtherBodyIndex :type Integer) (bFromSweep :type Boolean) (SweepResult :type Hit%20Result%20Structure%20%28by%20ref%29))
  (Utilities|Casting|CastToThirdPersonCharacter OtherActor)
  (if (not (Variables|Default|Get是否开灯))
    (Input|EnableInput (Game|GetPlayerController 0))
    (Rendering|SetVisibility (Variables|Default|GetTextRender) true false)
    (Utilities|FlowControl|Gate true) ; enters at Open
  ))

(event OnComponentEndOverlap(Box)
  (params (OverlappedComponent :type Primitive%20Component%20Object%20Reference) (OtherActor :type Actor%20Object%20Reference) (OtherComp :type Primitive%20Component%20Object%20Reference) (OtherBodyIndex :type Integer))
  (Utilities|Casting|CastToThirdPersonCharacter OtherActor)
  (Input|DisableInput (Game|GetPlayerController 0))
  (Rendering|SetVisibility (Variables|Default|GetTextRender) false false)
  (Utilities|FlowControl|Gate true) ; enters at Close
)

(event EventBeginPlay)

(event Collision|EventActorBeginOverlap
  (params (OtherActor :type Actor%20Object%20Reference)))

(event EventTick
  (params (DeltaSeconds :type Float%20%28single-precision%29)))

(event Input|KeyboardEvents|F
  (params (Key :type Key%20Structure))
  (:Pressed
    (Utilities|FlowControl|Gate true
      (:Exit
        (Rendering|SetVisibility (Variables|Default|GetSpotLight) true false)
        (Rendering|SetVisibility (Variables|Default|GetTextRender) false false)
        (Variables|Default|Set是否开灯 true)
        (bind _outactors (Actor|GetAllActorsOfClass "light_BP_C"))
        (bind _array_element (Utilities|Array|ForEachLoopwithBreak _outactors :!label _label)
          (:LoopBody
            (if (Variables|light_BP_C|Get是否开灯 _array_element)
              (Variables|Default|Set是否可以开启机关 true)
              (else
                (Variables|Default|Set是否可以开启机关 false)
                (goto _label Break))))
          (:Completed
            (if (Variables|Default|Get是否可以开启机关)
              (Development|ExecuteConsoleCommand "ce 打开关卡机关" 0))))))))

(fn ConstructionScript)